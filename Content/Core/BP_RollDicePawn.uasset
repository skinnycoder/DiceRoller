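; Pawn for dice rolling that spawns a tray, its configured dice and a row of grip recorders offset along its right vector.
; Each recorder gets a throw strength stepped between the minimum and maximum.
; Roll input throws the dice of the recorder closest to a fixed strength; a hard-coded branch bypasses rolling the pawn's own dice.
; Debug input toggles debug on both the pawn's and the recorders' dice.
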(event `self.ReceiveBeginPlay`
  (bind _returnvalue (`self.GetTransform`))
  (bind _rotation (.rotation _returnvalue))
  (`|SpawnActorFromClass` (`self.SourceTray`) _returnvalue "Undefined" "MultiplyWithRoot" null null)
  (for _array_element (`self.MyDice`)
    (bind _returnvalue_2 (`|SpawnActorFromClass` "/Game/Dice/BP_Die.BP_Die_C" _returnvalue "Undefined" "MultiplyWithRoot" null _array_element null))
    (`KismetArrayLibrary.Array_Add` (`self.Dice`) _returnvalue_2))
  (for _index (range (+ (`KismetMathLibrary.FTrunc` (/ (- (`self.MaxThrowStrength`) (`self.MinThrowStrength`)) (`self.ThrowIterator`))) 1))
    (bind _returnvalue_3 (`|SpawnActorFromClass` "/Game/Recorder/BP_GripRecorder.BP_GripRecorder_C" (`KismetMathLibrary.MakeTransform` (+ (.location _returnvalue) (* (`KismetMathLibrary.GetRightVector` _rotation) (* (+ _index 1) 1000.0))) _rotation (.scale _returnvalue)) "Undefined" "MultiplyWithRoot" null (make `/Game/Core/DiceThrow` (1.0 0.0 0.0) (+ (* _index (`self.ThrowIterator`)) (`self.MinThrowStrength`))) self))
    (`KismetArrayLibrary.Array_Add` (`self.Grip Recordings`) _returnvalue_3)))

(event `EnhancedInput|/Game/TopDown/Input/Actions/IA_Roll`
  (params (ActionValue :type Boolean) (ElapsedSeconds :type "Float (double-precision)") (TriggeredSeconds :type "Float (double-precision)") (InputAction :type "InputAction Object Reference" :default "/Game/TopDown/Input/Actions/IA_Roll.IA_Roll"))
  (bind _dicethrow (make `/Game/Core/DiceThrow` (1.0 0.0 0.0) 1600.0))
  (:`Started`
    (if false
      (for _array_element (`self.Dice`)
        (`/Game/Dice/BP_Die.Roll Die` _array_element _dicethrow))
      (else
        (bind _recording (`self.Get Best Recording` _dicethrow))
        (for _array_element_2 (`/Game/Recorder/BP_GripRecorder.Dice` _recording)
          (`/Game/Dice/BP_Die.Roll Die` _array_element_2 _dicethrow))))))

(event `EnhancedInput|/Game/TopDown/Input/Actions/IA_DebugToggle`
  (params (ActionValue :type Boolean) (ElapsedSeconds :type "Float (double-precision)") (TriggeredSeconds :type "Float (double-precision)") (InputAction :type "InputAction Object Reference" :default "/Game/TopDown/Input/Actions/IA_DebugToggle.IA_DebugToggle"))
  (:`Started`
    (for _array_element (`self.Dice`)
      (`/Game/Dice/BP_Die.Toggle Debug` _array_element))
    (for _array_element_2 (`self.Grip Recordings`)
      (for _array_element_3 (`/Game/Recorder/BP_GripRecorder.Dice` _array_element_2)
        (`/Game/Dice/BP_Die.Toggle Debug` _array_element_3)))))

(fn `Get Best Recording`
  (params (DiceThrow :type "/Game/Core/DiceThrow Structure"))
  (returns (Recording :type "/Game/Recorder/BP_GripRecorder Object Reference"))
  (locals (BestRecording :type "/Game/Recorder/BP_GripRecorder Object Reference") (ClosestThrow :type "Float (double-precision)" :default 99999999.0))
  (for _array_element (`self.Grip Recordings`)
    (bind _returnvalue (`KismetMathLibrary.Abs` (- (`.Strength_5_A090D9C1485D23BAF0BEEAA507284405` (break `/Game/Core/DiceThrow` (`/Game/Recorder/BP_GripRecorder.ThrowStrength` _array_element))) (`.Strength_5_A090D9C1485D23BAF0BEEAA507284405` (break `/Game/Core/DiceThrow` DiceThrow)))))
    (if (< _returnvalue (`local.ClosestThrow`))
      (set `local.ClosestThrow` _returnvalue)
      (set `local.BestRecording` _array_element)))
  (return (`local.BestRecording`)))

(fn `UserConstructionScript`)