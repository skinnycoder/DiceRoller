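; BP_GripRecorder is an actor that spawns a dice tray and throws the owning pawn's dice at its own transform.
; Its construction script casts the instigator to BP_RollDicePawn and caches it as OwningPawn.
; BeginPlay spawns the pawn's SourceTray class, then a BP_Die for each MyDice entry, passing that entry as DiceType.
; Each die is added to the Dice array and immediately rolled with ThrowStrength.
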(event `self.ReceiveBeginPlay`
  (`|SpawnActorFromClass` (`/Game/Core/BP_RollDicePawn.SourceTray` (`self.OwningPawn`)) (`self.GetTransform`) "Undefined" "MultiplyWithRoot" null null)
  (for _array_element (`/Game/Core/BP_RollDicePawn.MyDice` (`self.OwningPawn`))
    (bind _returnvalue (`|SpawnActorFromClass` "/Game/Dice/BP_Die.BP_Die_C" (`self.GetTransform`) "Undefined" "MultiplyWithRoot" null _array_element null))
    (`KismetArrayLibrary.Array_Add` (`self.Dice`) _returnvalue)
    (`/Game/Dice/BP_Die.Roll Die` _returnvalue (`self.ThrowStrength`))))

(fn `UserConstructionScript`
  (bind _asbp_roll_dice_pawn (cast `/Game/Core/BP_RollDicePawn` (`self.GetInstigator`)))
  (set `self.OwningPawn` _asbp_roll_dice_pawn))