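; BP_Die is a physics die whose recorded roll replays showing the maximum number.
; Construction pulls mesh, textures and side count from a data table row matching DiceType into a dynamic material.
; Rolls apply random impulses while RecorderAC records; when recording ends, the highest numbered mesh socket gives the result.
; On playback, the material's TopNumber remaps face numbers so that face shows the highest value, faking the outcome without changing the physics.
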(event `self.ReceiveBeginPlay`
  (bind _recorder_ac (`self.Recorder_AC`))
  (`|ExecutionSequence`
    (:`then_0`
      (bind _asbp_top_down_character (cast `/Game/TopDown/Blueprints/BP_TopDownCharacter` (`GameplayStatics.GetPlayerCharacter` 0)))
      (add `/Game/TopDown/Blueprints/BP_TopDownCharacter.ToggleDebug` _asbp_top_down_character (delegate `OnToggleDebug`))
      (add `/Game/TopDown/Blueprints/BP_TopDownCharacter.RollDice` _asbp_top_down_character (delegate `OnRollDice`))
      (add `/Game/Recorder/Recorder_AC.OnPlaybackEnd` _recorder_ac (delegate `OnPlaybackEnd`))
      (add `/Game/Recorder/Recorder_AC.OnPlaybackBegin` _recorder_ac (delegate `OnPlaybackStart`))
      (add `/Game/Recorder/Recorder_AC.OnRecordEnd` _recorder_ac (delegate `OnRecordEnd`)))
    (:`then_1`
      (`KismetSystemLibrary.Delay` 0.2)
      (`self.Roll Die`))))

(event `OnPlaybackEnd`)

(event `OnToggleDebug`
  (set `self.DebugOn` (not (`self.DebugOn`))))

(event `OnRollDice`
  (`self.Roll Die`))

(event `OnPlaybackStart`
  (`self.Change Future Roll` (`self.Get Number Of Sides`)))

(event `OnRecordEnd`
  (bind _value (`self.Calc Roll Based on Socket`))
  (bind _output_get (set `self.ActualNumber` _value))
  (set `self.TargetValue` _output_get))

(event `self.ReceiveTick`
  (params (DeltaSeconds :type "Float (single-precision)"))
  (`KismetSystemLibrary.PrintString` "Space/[A]: Roll the Dice \nCtrl/[B]: Replay the Dice (MAX ROLL!) \nD/[Select[]: Toggle Debugging" true false (struct :`R` 1.0 :`G` 0.809113 :`B` 0.011239 :`A` 1.0) 2.0 "Keybinds")
  (`self.Calc Roll Based on Socket`)
  (switch `/Game/Dice/DieState` (`self.State`)))

(event `self.Die.OnComponentHit`
  (params (HitComponent :type "PrimitiveComponent Object Reference") (OtherActor :type "Actor Object Reference") (OtherComp :type "PrimitiveComponent Object Reference") (NormalImpulse :type "Vector Structure") (Hit :type "HitResult Structure (by ref)"))
  (if (> (- (`KismetSystemLibrary.GetGameTimeInSeconds`) (`self.LastCollisionTime`)) (`self.CollisionCooldown`))
    (bind _returnvalue (`PrimitiveComponent.GetPhysicsLinearVelocity` HitComponent "None"))
    (bind _returnvalue_2 (`KismetMathLibrary.VSize` _returnvalue))
    (`GameplayStatics.PlaySoundAtLocation` "/Game/Dice/Sounds/DieCollision_Cue.DieCollision_Cue" (`.ImpactPoint` (`GameplayStatics.BreakHitResult` Hit)) (struct) (`KismetMathLibrary.MapRangeClamped` _returnvalue_2 25.0 500.0 0.0 1.0) (`KismetMathLibrary.MapRangeClamped` _returnvalue_2 15.0 500.0 0.5 1.0) 0.0 null null null null)
    (set `self.LastCollisionTime` (`KismetSystemLibrary.GetGameTimeInSeconds`))))

(event `Roll Die`
  (bind _die (`self.Die`))
  (`self.K2_SetActorTransform` (`self.StartTransform`) false true)
  (`PrimitiveComponent.AddImpulse` _die (`KismetMathLibrary.MakeVector` (`KismetMathLibrary.RandomFloatInRange` 1600.0 2000.0)) "None" true)
  (`PrimitiveComponent.AddAngularImpulseInRadians` _die (* (`KismetMathLibrary.GreaterGreater_VectorRotator` (`KismetMathLibrary.MakeVector` 1.0) (`KismetMathLibrary.MakeRotator` (`KismetMathLibrary.RandomFloatInRange` 0.0 360.0) (`KismetMathLibrary.RandomFloatInRange` 0.0 360.0) (`KismetMathLibrary.RandomFloatInRange` 0.0 360.0))) 20.0) "None" true)
  (`/Game/Recorder/Recorder_AC.StartRecording` (`self.Recorder_AC`)))

(fn `Calc Roll Based on Collision`
  (returns (Value :type Integer))
  (bind _returnvalue (`self.K2_GetActorLocation`))
  (bind _returnvalue_x (`KismetMathLibrary.BreakVector` (`self.GetActorScale3D`)))
  (bind _debugcolor (`/Game/Recorder/Recorder_AC.DebugColor` (`self.Recorder_AC`)))
  (bind _returnvalue_2 (+ _returnvalue (* (`KismetMathLibrary.MakeVector` 0.0 0.0 -1.0) 150.0 _returnvalue_x)))
  (bind (_outhit _returnvalue_3) (`KismetSystemLibrary.LineTraceSingle` _returnvalue _returnvalue_2 "TraceTypeQuery1" false (`|MakeArray` self :!type "Actor Object Reference")))
  (`KismetSystemLibrary.DrawDebugLine` _returnvalue _returnvalue_2 _debugcolor)
  (bind _returnvalue_4 (`KismetMathLibrary.SelectVector` (`.Normal` (`GameplayStatics.BreakHitResult` _outhit)) (0.0 0.0 1.0) _returnvalue_3))
  (bind _returnvalue_5 (+ _returnvalue (* _returnvalue_4 150.0 _returnvalue_x 2.0)))
  (`KismetSystemLibrary.DrawDebugLine` _returnvalue _returnvalue_5 _debugcolor 0.0 2.5)
  (`KismetSystemLibrary.DrawDebugString` (+ _returnvalue_5 (* _returnvalue_4 15.0)) "3" null _debugcolor))

(fn `Calc Roll Based on Socket`
  (returns (Value :type Integer))
  (locals (HighestZ :type "Float (double-precision)" :default -999999999.0) (RolledNumber :type Integer) (HighestSocket :type Name :default "None"))
  (bind _returnvalue (`self.K2_GetActorLocation`))
  (bind _returnvalue_x (`KismetMathLibrary.BreakVector` (`self.GetActorScale3D`)))
  (bind _targetvalue (`self.TargetValue`))
  (bind _returnvalue_2 (`KismetStringLibrary.Conv_IntToString` (`local.RolledNumber`)))
  (bind _returnvalue_3 (* (`self.ComplimentaryColor`) 10.0))
  (bind _returnvalue_4 (+ _returnvalue (* (`KismetMathLibrary.Normal` (- (`SceneComponent.GetSocketLocation` (`self.Die`) (`local.HighestSocket`)) _returnvalue)) 150.0 _returnvalue_x)))
  (for _index (range 1 (+ (`self.Get Number Of Sides`) 1))
    (bind _returnvalue_5 (`KismetStringLibrary.Conv_StringToName` (`KismetStringLibrary.Conv_IntToString` _index)))
    (bind _returnvalue_6 (`StaticMesh.FindSocket` (`StaticMeshComponent.StaticMesh` (`self.Die`)) _returnvalue_5))
    (`/Engine/EditorBlueprintResources/StandardMacros.IsValid` _returnvalue_6
      (:`Is Valid`
        (bind _z (.z (`KismetMathLibrary.TransformLocation` (`self.GetTransform`) (`StaticMeshSocket.RelativeLocation` _returnvalue_6))))
        (if (> _z (`local.HighestZ`))
          (set `local.HighestZ` _z)
          (set `local.RolledNumber` _index)
          (set `local.HighestSocket` _returnvalue_5)))))
  (`|ExecutionSequence`
    (:`then_0`
      (if (`self.DebugOn`)
        (`KismetSystemLibrary.DrawDebugLine` _returnvalue _returnvalue_4 _returnvalue_3 0.0 1.0)
        (`KismetSystemLibrary.DrawDebugString` (+ _returnvalue_4 (`KismetMathLibrary.MakeVector` 0.0 0.0 15.0)) (`KismetMathLibrary.SelectString` _returnvalue_2 (`KismetStringLibrary.Concat_StrStr` _returnvalue_2 " -> " (`KismetStringLibrary.Conv_IntToString` _targetvalue)) (== _targetvalue (`self.ActualNumber`))) null _returnvalue_3)))
    (:`then_1`
      (return (`local.RolledNumber`)))))

(fn `Calc Top Number`
  (returns (TopNumber :type "Float (double-precision)"))
  (locals (AdjustedActual :type Integer))
  (bind _actualnumber (`self.ActualNumber`))
  (bind _returnvalue (/ (`self.Get Number Of Sides`) 2))
  (bind _returnvalue_2 (+ (`self.Get Number Of Sides`) 1))
  (bind _returnvalue_3 (> _actualnumber _returnvalue))
  (bind _returnvalue_4 (> (`self.TargetValue`) _returnvalue))
  (bind _returnvalue_5 (== (mod (`self.TargetValue`) 2) 0))
  (bind _output_get (set `local.AdjustedActual` (`KismetMathLibrary.SelectInt` (- _returnvalue_2 _actualnumber) _actualnumber _returnvalue_3)))
  (bind _returnvalue_6 (+ (+ (select `bool` _returnvalue_4 :`false` (- 1 _output_get) :`true` (+ (- _returnvalue 1) _output_get)) (`self.TargetValue`)) (* (`KismetMathLibrary.SelectInt` 2 0 (and (== (mod _output_get 2) 0) (select `bool` _returnvalue_4 :`false` (not _returnvalue_5) :`true` _returnvalue_5))) (`KismetMathLibrary.SelectInt` -1 1 _returnvalue_5))))
  (return (`KismetMathLibrary.Conv_IntToDouble` (`KismetMathLibrary.SelectInt` (- _returnvalue_2 _returnvalue_6) _returnvalue_6 _returnvalue_3))))

(fn `Change Future Roll`
  (params (ForcedRoll :type Integer))
  (set `self.TargetValue` ForcedRoll)
  (`MaterialInstanceDynamic.SetScalarParameterValue` (`self.DiceMaterial`) "TopNumber" (`self.Calc Top Number`)))

(fn `Get Number Of Sides`
  (returns (NumSides :type Integer))
  (return (`.NumSides_5_24DA1957467C86FE04D35FA8CCBF18E7` (break `/Game/Dice/DiceParams` (`self.DiceParams`)))))

(fn `Init Die Data`
  (bind (_dicetype _numsides _staticmesh _texture _normal) (break `/Game/Dice/DiceParams` (`self.DiceParams`)))
  (bind _outrownames (`DataTableFunctionLibrary.GetDataTableRowNames` "/Game/Dice/DiceDataTable.DiceDataTable"))
  (for _array_element _outrownames
    (bind _returnvalue (`|GetDataTableRow` "/Game/Dice/DiceDataTable.DiceDataTable" _array_element)
      (:`then`
        (if (`|EnumEquality` (`.DiceType_2_0A34EBF44C306001750618A504703FE8` (break `/Game/Dice/DiceParams` _returnvalue)) (`self.DiceType`))
          (set `self.DiceParams` _returnvalue)
          (break)))))
  (`StaticMeshComponent.SetStaticMesh` (`self.Die`) _staticmesh)
  (bind _returnvalue_2 (`PrimitiveComponent.CreateDynamicMaterialInstance` (`self.Die`) 0 null "None"))
  (bind _output_get (set `self.DiceMaterial` _returnvalue_2))
  (`MaterialInstanceDynamic.SetScalarParameterValue` _output_get "NumberOfSides" (`KismetMathLibrary.Conv_IntToDouble` _numsides))
  (`MaterialInstanceDynamic.SetTextureParameterValue` _output_get "DiceNumberNormals" _normal)
  (`MaterialInstanceDynamic.SetTextureParameterValue` _output_get "DiceNumberTexture" _texture)
  (`self.Update Dice Faces`)
  (`self.Init Die Material`))

(fn `Init Die Material`
  (locals (Hue :type "Float (double-precision)" :default 0.0))
  (bind _dicematerial (`self.DiceMaterial`))
  (`MaterialInstanceDynamic.SetVectorParameterValue` _dicematerial "DieColor1" (`self.PrimaryColor`))
  (`MaterialInstanceDynamic.SetVectorParameterValue` _dicematerial "DieColor2" (`self.ComplimentaryColor`)))

(fn `Save Start Transform`
  (set `self.StartTransform` (`self.GetTransform`)))

(fn `Update Dice Faces`
  (`MaterialInstanceDynamic.SetScalarParameterValue` (`self.DiceMaterial`) "TopNumber" (`self.Calc Top Number`)))

(fn `UserConstructionScript`
  (`self.Save Start Transform`)
  (`self.Init Die Data`))

(fn `Weight Dice To Side (WIP)`
  (params (Side :type Integer))
  (`PrimitiveComponent.SetCenterOfMass` (`self.Die`) (* (- (`SceneComponent.GetSocketLocation` (`self.Die`) (`KismetStringLibrary.Conv_StringToName` (`KismetStringLibrary.Conv_IntToString` Side))) (`self.K2_GetActorLocation`)) 1.0) "None"))